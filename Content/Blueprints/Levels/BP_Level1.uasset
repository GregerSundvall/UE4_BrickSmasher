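; BP_Level1 is a level actor that holds a layout of 24 bricks as child actor components.
; On BeginPlay it casts each child actor to GBrick, registers itself as the parent level and collects it in the Bricks array.
; Tick prints the array's length as debug output.
; Macros for delayed brick visibility toggling exist, but the staggered loop in the event graph is disconnected and never runs.
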(event `self.ReceiveBeginPlay`
  (for _array_element (`|MakeArray` (`self.Brick1`) (`self.Brick2`) (`self.Brick3`) (`self.Brick4`) (`self.Brick5`) (`self.Brick6`) (`self.Brick7`) (`self.Brick8`) (`self.Brick9`) (`self.Brick10`) (`self.Brick11`) (`self.Brick12`) (`self.Brick13`) (`self.Brick14`) (`self.Brick15`) (`self.Brick16`) (`self.Brick17`) (`self.Brick18`) (`self.Brick19`) (`self.Brick20`) (`self.Brick21`) (`self.Brick22`) (`self.Brick23`) (`self.Brick24`) :!type "SceneComponent Object Reference")
    (bind _aschild_actor_component (cast `ChildActorComponent` _array_element))
    (bind _asgbrick (cast `GBrick` (`ChildActorComponent.ChildActor` _aschild_actor_component)))
    (`GBrick.SetParentLevel` _asgbrick self)
    (`KismetArrayLibrary.Array_Add` (`self.Bricks`) _asgbrick)))

(event `self.ReceiveTick`
  (params (DeltaSeconds :type "Float (single-precision)"))
  (`KismetSystemLibrary.PrintString` (`KismetStringLibrary.Conv_IntToString` (`KismetArrayLibrary.Array_Length` (`self.Bricks`)))))

(fn `UserConstructionScript`)