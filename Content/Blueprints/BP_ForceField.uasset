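; BP_ForceField is a force field actor that animates three bolt components to look erratic, with no gameplay logic.
; Every Tick, each bolt runs through Vibrate, then Rotate with its own maximum turning speed.
; Vibrate teleports the bolt to a random delta-time-scaled offset around its parent-relative origin, so it jitters without drifting.
; Rotate adds a random, positive local pitch, also scaled by delta time.
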(event `self.ReceiveTick`
  (params (DeltaSeconds :type "Float (single-precision)"))
  (bind _bolt3 (`self.Bolt3`))
  (bind _bolt1 (`self.Bolt1`))
  (bind _bolt2 (`self.Bolt2`))
  (`self.Vibrate` _bolt1)
  (`self.Rotate` _bolt1 2000.0)
  (`self.Vibrate` _bolt2)
  (`self.Rotate` _bolt2 400.0)
  (`self.Vibrate` _bolt3)
  (`self.Rotate` _bolt3 600.0))

(fn `NewFunction_0`)

(fn `UserConstructionScript`)